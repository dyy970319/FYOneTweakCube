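; One cube piece, apparently from a Rubik's-style puzzle, built from FYOneFace child actors, with a touched flag.
; ResetMaterial takes a rotation axis index and direction, and SortFace orders the four faces around that axis forward or reversed.
; It then shifts the plane materials one step around that ring and zeroes the cube's world rotation, so turns persist as material swaps rather than accumulated rotation.
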(fn `getIsTouched`
  (returns (NewParam :type Boolean))
  (return (`self.isTouched`)))

(fn `Reset Material`
  (params (mRotateFrag :type Integer) (mRotateDirection :type Boolean))
  (locals (tempMaterial :type "MaterialInterface Object Reference") (tempFYOneFace :type "Array of ChildActorComponent Object Reference"))
  (bind _tempfyoneface (`local.tempFYOneFace`))
  (switch `int` mRotateFrag
    (:`0`
      (`self.sortFace` (`self.FYOneFace`) (`self.FYOneFace3`) (`self.FYOneFace1`) (`self.FYOneFace2`) (`local.tempFYOneFace`) (== mRotateDirection false)))
    (:`1`
      (`self.sortFace` (`self.FYOneFace`) (`self.FYOneFace4`) (`self.FYOneFace1`) (`self.FYOneFace5`) (`local.tempFYOneFace`) (== mRotateDirection true)))
    (:`2`
      (`self.sortFace` (`self.FYOneFace2`) (`self.FYOneFace4`) (`self.FYOneFace3`) (`self.FYOneFace5`) (`local.tempFYOneFace`) (== mRotateDirection false))))
  (bind _asfyone_face (cast `/Game/Blueprints/FYOneFace` (`ChildActorComponent.ChildActor` (`|GetArrayItem` _tempfyoneface))))
  (bind _plane (`/Game/Blueprints/FYOneFace.Plane` _asfyone_face))
  (set `local.tempMaterial` (`PrimitiveComponent.GetMaterial` _plane 0))
  (bind _asfyone_face_2 (cast `/Game/Blueprints/FYOneFace` (`ChildActorComponent.ChildActor` (`|GetArrayItem` _tempfyoneface 1))))
  (bind _plane_2 (`/Game/Blueprints/FYOneFace.Plane` _asfyone_face_2))
  (`PrimitiveComponent.SetMaterial` _plane 0 (`PrimitiveComponent.GetMaterial` _plane_2 0))
  (bind _asfyone_face_3 (cast `/Game/Blueprints/FYOneFace` (`ChildActorComponent.ChildActor` (`|GetArrayItem` _tempfyoneface 2))))
  (bind _plane_3 (`/Game/Blueprints/FYOneFace.Plane` _asfyone_face_3))
  (`PrimitiveComponent.SetMaterial` _plane_2 0 (`PrimitiveComponent.GetMaterial` _plane_3 0))
  (bind _asfyone_face_4 (cast `/Game/Blueprints/FYOneFace` (`ChildActorComponent.ChildActor` (`|GetArrayItem` _tempfyoneface 3))))
  (bind _plane_4 (`/Game/Blueprints/FYOneFace.Plane` _asfyone_face_4))
  (`PrimitiveComponent.SetMaterial` _plane_3 0 (`PrimitiveComponent.GetMaterial` _plane_4 0))
  (`PrimitiveComponent.SetMaterial` _plane_4 0 (`local.tempMaterial`))
  (`SceneComponent.K2_SetWorldRotation` :`self` (`self.Cube`)))

(fn `setIsTouched`
  (params (NewParam :type Boolean))
  (set `self.isTouched` NewParam))

(fn `sortFace`
  (params (childActor :type "ChildActorComponent Object Reference (by ref)") (childActor2 :type "ChildActorComponent Object Reference (by ref)") (childActor3 :type "ChildActorComponent Object Reference (by ref)") (childActor4 :type "ChildActorComponent Object Reference (by ref)") (childActorArray :type "Array of ChildActorComponent Object Reference (by ref)") (direction :type "Boolean (by ref)"))
  (bind _returnvalue (`KismetArrayLibrary.Array_Length` childActorArray))
  (`KismetArrayLibrary.Array_Clear` childActorArray)
  (if direction
    (`KismetArrayLibrary.Array_Insert` childActorArray childActor)
    (`KismetArrayLibrary.Array_Insert` childActorArray childActor2)
    (`KismetArrayLibrary.Array_Insert` childActorArray childActor3)
    (`KismetArrayLibrary.Array_Insert` childActorArray childActor4)
    (else
      (`KismetArrayLibrary.Array_Insert` childActorArray childActor _returnvalue)
      (`KismetArrayLibrary.Array_Insert` childActorArray childActor2 _returnvalue)
      (`KismetArrayLibrary.Array_Insert` childActorArray childActor3 _returnvalue)
      (`KismetArrayLibrary.Array_Insert` childActorArray childActor4 _returnvalue))))

(fn `UserConstructionScript`)