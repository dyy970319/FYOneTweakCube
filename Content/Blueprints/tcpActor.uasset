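; TCP client actor that exchanges player time records with a hardcoded remote server, connecting on BeginPlay.
; GetTime, UpdateTime and GetTopTimes send string-encoded requests led by an opcode, adding length-prefixed names and time where needed.
; Replies route by the last stored OperationType, with only GetTime's stored as best time in FYGameInstance.
; GetTopTimes leaves OperationType unchanged and has no reply handling; the Disconnect call is unwired.
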(event `self.ReceiveBeginPlay`
  (bind _connectionid (`self.Connect` "152.136.96.110" 2047 (delegate `Disconnected`) (delegate `Connected`) (delegate `ReceivedMessage`)))
  (set `self.socket connect` _connectionid))

(event `Disconnected`
  (params (ConnectionId :type Integer))
  (`KismetSystemLibrary.PrintString` "disconnectd"))

(event `Connected`
  (params (ConnectionId :type Integer))
  (`KismetSystemLibrary.PrintString` "connected"))

(event `ReceivedMessage`
  (params (ConnectionId :type Integer) (Message :type "Array of Byte (by ref)"))
  (bind _operationtype (`self.operationType`))
  (bind _localbytearr (`self.localByteArr`))
  (set `self.localByteArr` Message)
  (if (== _operationtype 0)
    _
    (elif (== _operationtype 1)
      (bind _returnvalue (`self.Message_ReadString` _localbytearr (`KismetArrayLibrary.Array_Length` _localbytearr)))
      (bind _asfygame_instance (cast `/Game/Blueprints/FYGameInstance` (`GameplayStatics.GetGameInstance`)))
      (set `/Game/Blueprints/FYGameInstance.gBestPlayerTime` (`KismetStringLibrary.Conv_StringToDouble` _returnvalue) _asfygame_instance)
      (`KismetSystemLibrary.PrintString` "received message"))))

(fn `getTime`
  (bind _asfygame_instance (cast `/Game/Blueprints/FYGameInstance` (`GameplayStatics.GetGameInstance`)))
  (set `self.operationType` 1)
  (bind _gplayername (`/Game/Blueprints/FYGameInstance.gPlayerName` _asfygame_instance))
  (`self.SendData` (`self.socket connect`) (`self.Concat_BytesBytes` (`self.Conv_StringToBytes` (`KismetStringLibrary.Conv_IntToString` 1)) (`self.Conv_StringToBytes` (`KismetStringLibrary.Conv_IntToString` (`KismetStringLibrary.Len` _gplayername))) (`self.Conv_StringToBytes` _gplayername))))

(fn `getTopTimes`
  (`self.SendData` (`self.socket connect`) (`self.Conv_StringToBytes` (`KismetStringLibrary.Conv_IntToString` 2))))

(fn `updateTime`
  (params (inputName :type String) (inputTime :type "Float (double-precision)"))
  (set `self.operationType` 0)
  (`self.SendData` (`self.socket connect`) (`self.Concat_BytesBytes` (`self.Conv_StringToBytes` (`KismetStringLibrary.Conv_IntToString` 0)) (`self.Conv_StringToBytes` (`KismetStringLibrary.Conv_IntToString` (`KismetStringLibrary.Len` inputName))) (`self.Conv_StringToBytes` inputName) (`self.Conv_StringToBytes` (`KismetStringLibrary.Conv_DoubleToString` inputTime)))))

(fn `UserConstructionScript`)