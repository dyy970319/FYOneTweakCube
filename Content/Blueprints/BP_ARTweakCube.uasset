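; Rubik's cube puzzle actor, named for AR, that builds 27 child cubes on construction and scrambles them with random instant turns.
; TouchRotate infers axis, layer and direction from two touched pieces, then Tick turns the nine matching cubes around their averaged center.
; Each finished turn resets cube materials and compares face materials per side.
; A solved cube hides, spawns a random effect and, for long scrambles, reports player time through TcpActor.
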(event `self.ReceiveTick`
  (params (DeltaSeconds :type "Float (single-precision)"))
  (bind _angleself (`self.angleSelf`))
  (if (< _angleself 90.0)
    (set `self.angleSelf` (+ _angleself (`self.increaseNum`)))
    (`self.rotateNineCubes`)))

(fn `clearTouchArray`
  (for _array_element (`self.touchArray`)
    (`/Game/Blueprints/FYOneCube.setIsTouched` _array_element false))
  (set `self.touchArray` (`self.zeroArr`)))

(fn `correctRotate`
  (params (NewParam :type "Float (double-precision)"))
  (returns (NewParam1 :type "Float (double-precision)"))
  (locals (NewLocalVar_0 :type Boolean))
  (bind (_newparam2 _newparam3) (`self.nearlyReturnValue` NewParam))
  (if (== _newparam3 true)
    (return _newparam2)
    (else
      (bind (_newparam2_2 _newparam3_2) (`self.nearlyReturnValue` NewParam 90.0))
      (if (== _newparam3_2 true)
        (return _newparam2_2)
        (else
          (bind (_newparam2_3 _newparam3_3) (`self.nearlyReturnValue` NewParam -90.0))
          (if (== _newparam3_3 true)
            (return _newparam2_3)
            (else
              (bind (_newparam2_4 _newparam3_4) (`self.nearlyReturnValue` NewParam 180.0))
              (if (== _newparam3_4 true)
                (return _newparam2_4)
                (else
                  (bind (_newparam2_5 _newparam3_5) (`self.nearlyReturnValue` NewParam -180.0))
                  (if (== _newparam3_5 true)
                    (return _newparam2_5)
                    (else
                      (bind (_newparam2_6 _newparam3_6) (`self.nearlyReturnValue` 0.0 270.0))
                      (if (== _newparam3_6 true)
                        (return _newparam2_6)
                        (else
                          (bind (_newparam2_7 _newparam3_7) (`self.nearlyReturnValue` 0.0 -270.0))
                          (if (== _newparam3_7 true)
                            (return _newparam2_7)
                            (else
                              (return NewParam))))))))))))))))

(fn `getFaceByIndex`
  (params (cube :type "/Game/Blueprints/FYOneCube Object Reference") (index :type Integer))
  (returns (NewParam :type "ChildActorComponent Object Reference"))
  (locals (tempCube :type "/Game/Blueprints/FYOneCube Object Reference"))
  (bind _tempcube (`local.tempCube`))
  (set `local.tempCube` cube)
  (switch `int` index
    (:`0`
      (return (`/Game/Blueprints/FYOneCube.FYOneFace` _tempcube)))
    (:`1`
      (return (`/Game/Blueprints/FYOneCube.FYOneFace1` _tempcube)))
    (:`2`
      (return (`/Game/Blueprints/FYOneCube.FYOneFace2` _tempcube)))
    (:`3`
      (return (`/Game/Blueprints/FYOneCube.FYOneFace3` _tempcube)))
    (:`4`
      (return (`/Game/Blueprints/FYOneCube.FYOneFace4` _tempcube)))
    (:`5`
      (return (`/Game/Blueprints/FYOneCube.FYOneFace5` _tempcube)))))

(fn `getLineNum`
  (params (pos :type "Float (double-precision)"))
  (returns (returnLineNum :type Integer))
  (if (< pos (- 0.0 (`self.distance`)))
    (return 0)
    (elif (< pos (`self.distance`))
      (return 1)
      (else
        (return 2)))))

(fn `getStartPosition`
  (params (direction :type Integer) (index :type Integer))
  (returns (startPosition :type "Vector Structure"))
  (bind _returnvalue (- index 1))
  (bind _distance (`self.distance`))
  (switch `int` direction
    (:`0`
      (return (* (`KismetMathLibrary.MakeVector` _distance) _returnvalue)))
    (:`1`
      (return (* (`KismetMathLibrary.MakeVector` 0.0 _distance) _returnvalue)))
    (:`2`
      (return (* (`KismetMathLibrary.MakeVector` 0.0 0.0 _distance) _returnvalue)))))

(fn `getTouchRotateDirection`
  (returns (NewParam :type Boolean))
  (bind _rotatedirection (`/Game/Blueprints/FYOneCube.rotateDirection` (`|GetArrayItem` (`self.touchArray`))))
  (bind (_returnvalue_x _returnvalue_y _returnvalue_z) (`KismetMathLibrary.BreakVector` (`SceneComponent.K2_GetComponentLocation` (`/Game/Blueprints/FYOneCube.Cube` (`|GetArrayItem` (`self.touchArray`))))))
  (bind _returnvalue (- (`SceneComponent.K2_GetComponentLocation` (`/Game/Blueprints/FYOneCube.Cube` (`|GetArrayItem` (`self.touchArray`)))) (`SceneComponent.K2_GetComponentLocation` (`/Game/Blueprints/FYOneCube.Cube` (`|GetArrayItem` (`self.touchArray`) 1)))))
  (bind _returnvalue_2 (`KismetMathLibrary.Vector_GetAbsMax` _returnvalue))
  (bind _output_get (set `self.tempVec` _returnvalue))
  (if (== (`KismetMathLibrary.Abs` (.x _output_get)) _returnvalue_2)
    (if (== (`/Game/Blueprints/FYOneCube.rotateDirection` (`|GetArrayItem` (`self.touchArray`))) 2)
      (return (> (* (.x _output_get) _returnvalue_z) 0.0))
      (else
        (return (< (* _returnvalue_y (.x _output_get)) 0.0))))
    (elif (== (`KismetMathLibrary.Abs` (.y _output_get)) _returnvalue_2)
      (if (== _rotatedirection 0)
        (return (> (* _returnvalue_x (.y _output_get)) 0.0))
        (else
          (return (< (.y _output_get) 0.0))))
      (elif (== _rotatedirection 1)
        (return (> (* _returnvalue_y (.z _output_get)) 0.0))
        (else
          (return (< (* (.z _output_get) _returnvalue_x) 0.0)))))))

(fn `isPosRight`
  (params (cube :type "/Game/Blueprints/FYOneCube Object Reference") (index :type Integer))
  (returns (NewParam1 :type Boolean))
  (locals (tempX :type "Float (double-precision)" :default 0.0) (tempY :type "Float (double-precision)" :default 0.0) (tempZ :type "Float (double-precision)" :default 0.0))
  (bind _tempz (`local.tempZ`))
  (bind _tempx (`local.tempX`))
  (bind _tempy (`local.tempY`))
  (bind (_returnvalue_x _returnvalue_y _returnvalue_z) (`KismetMathLibrary.BreakVector` (`SceneComponent.K2_GetComponentLocation` (`/Game/Blueprints/FYOneCube.Cube` cube))))
  (set `local.tempX` _returnvalue_x)
  (set `local.tempY` _returnvalue_y)
  (set `local.tempZ` _returnvalue_z)
  (switch `int` index
    (:`0`
      (return (> _tempz 2.0)))
    (:`1`
      (return (< _tempz -2.0)))
    (:`2`
      (return (> _tempy 2.0)))
    (:`3`
      (return (< _tempy -2.0)))
    (:`4`
      (return (> _tempx 2.0)))
    (:`5`
      (return (< _tempx -2.0)))))

(fn `isRotateRight`
  (returns (NewParam :type Boolean))
  (locals (tempFaceActorArray :type "Array of /Game/Blueprints/FYOneFace Object Reference") (tempMaterial :type "MaterialInterface Object Reference") (NullMaterial :type "MaterialInterface Object Reference"))
  (for _index (range 6)
    (for _array_element (`self.cubeArray`)
      (bind _newparam1 (`self.isPosRight` _array_element _index))
      (if _newparam1
        (bind _newparam (`self.getFaceByIndex` _array_element _index))
        (bind _asfyone_face (cast `/Game/Blueprints/FYOneFace` (`ChildActorComponent.ChildActor` _newparam)))
        (if (== (`local.tempMaterial`) (`local.NullMaterial`))
          (bind _returnvalue (`PrimitiveComponent.GetMaterial` (`/Game/Blueprints/FYOneFace.Plane` _asfyone_face) 0))
          (set `local.tempMaterial` _returnvalue)
          (elif (not (== (`local.tempMaterial`) _returnvalue))
            (set `local.tempMaterial` (`local.NullMaterial`))
            (return false)))))
    (set `local.tempMaterial` (`local.NullMaterial`)))
  (return true))

(fn `nearlyReturnValue`
  (params (NewParam :type "Float (double-precision)") (NewParam1 :type "Float (double-precision)"))
  (returns (NewParam2 :type "Float (double-precision)") (NewParam3 :type Boolean))
  (if (`KismetMathLibrary.NearlyEqual_FloatFloat` NewParam NewParam1 1.0)
    (return NewParam1 true)
    (else
      (return NewParam false))))

(fn `randomRotate`
  (bind _asfygame_instance (cast `/Game/Blueprints/FYGameInstance` (`GameplayStatics.GetGameInstance`)))
  (set `self.increaseNum` 90.0)
  (for _ (range 1 (+ (`/Game/Blueprints/FYGameInstance.gGameRandomTimes` _asfygame_instance) 1))
    (`self.startRotateCube` (`KismetMathLibrary.RandomIntegerInRange` 0 2) (`KismetMathLibrary.RandomBool`) (`KismetMathLibrary.RandomIntegerInRange` 0 2))
    (set `self.angleSelf` 90.0)
    (`self.rotateNineCubes`))
  (bind _asfygame_instance_2 (cast `/Game/Blueprints/FYGameInstance` (`GameplayStatics.GetGameInstance`)))
  (set `self.increaseNum` (`KismetMathLibrary.Conv_IntToDouble` (`/Game/Blueprints/FYGameInstance.gGameCubeMoveSpeed` _asfygame_instance_2))))

(fn `rotateNineCubes`
  (locals (cubeRelativeRotation :type "Rotator Structure" :default (struct)) (CubeRelativeRotationArray :type "Array of Rotator Structure") (NewLocalVar_0 :type "Rotator Structure" :default (struct :`Pitch` 89.0)))
  (bind (_cuberelativerotation_roll _cuberelativerotation_pitch _cuberelativerotation_yaw) (`KismetMathLibrary.BreakRotator` (`local.cubeRelativeRotation`)))
  (bind _rotatearray (`self.rotateArray`))
  (bind _returnvalue (* (`self.mRotateDirection`) (`self.distance`)))
  (bind _returnvalue_2 (* (- 0.0 (`KismetMathLibrary.Conv_IntToDouble` (`self.mRotateDirection`))) (`self.increaseNum`)))
  (`self.setRotateArray`)
  (for _array_element (`self.rotateArray`)
    (bind _cube (`/Game/Blueprints/FYOneCube.Cube` _array_element))
    (set `local.cubeRelativeRotation` (`SceneComponent.K2_GetComponentRotation` _cube))
    (switch `int` (`self.rotateFrag`)
      (:`0`
        (set `self.mRotateAxis` (`KismetMathLibrary.MakeVector` _returnvalue))
        (set `self.mRotateNew` (`KismetMathLibrary.MakeRotator` (+ _cuberelativerotation_roll _returnvalue_2))))
      (:`1`
        (set `self.mRotateAxis` (`KismetMathLibrary.MakeVector` 0.0 _returnvalue))
        (set `self.mRotateNew` (`KismetMathLibrary.MakeRotator` 0.0 (+ _cuberelativerotation_pitch _returnvalue_2))))
      (:`2`
        (set `self.mRotateAxis` (`KismetMathLibrary.MakeVector` 0.0 0.0 _returnvalue))
        (set `self.mRotateNew` (`KismetMathLibrary.MakeRotator` 0.0 0.0 (+ _cuberelativerotation_yaw (* (`self.mRotateDirection`) (`self.increaseNum`)))))))
    (`SceneComponent.K2_SetWorldLocation` _cube (+ (`self.centerPos`) (`KismetMathLibrary.RotateAngleAxis` (- (`SceneComponent.K2_GetComponentLocation` _cube) (`self.centerPos`)) (* 1.0 (`self.increaseNum`)) (`self.mRotateAxis`))) false false)
    (`SceneComponent.K2_SetWorldRotation` _cube (`self.mRotateNew`) false false))
  (if (`KismetMathLibrary.NearlyEqual_FloatFloat` (`self.angleSelf`) 90.0 0.0)
    (for _array_element_2 _rotatearray
      (`/Game/Blueprints/FYOneCube.Reset Material` _array_element_2 (`self.rotateFrag`) (== (`self.mRotateDirection`) -1)))
    (set `self.bIsRotating` false)
    (bind _newparam (`self.isRotateRight`))
    (if _newparam
      (`KismetSystemLibrary.PrintString` "还原成功")
      (`self.SetActorHiddenInGame` true)
      (switch `int` (`KismetMathLibrary.RandomIntegerInRange` 0 2)
        (:`0`
          (set `self.winParicle` "/Game/GrenadePack/Particles/VFX_GrenadeEXP_air.VFX_GrenadeEXP_air"))
        (:`1`
          (set `self.winParicle` "/Game/GrenadePack/Particles/VFX_GrenadeEXP_water.VFX_GrenadeEXP_water"))
        (:`2`
          (set `self.winParicle` "/Game/GrenadePack/Particles/VFX_LTGrenadeEXP_wood.VFX_LTGrenadeEXP_wood")))
      (`GameplayStatics.SpawnEmitterAtLocation` (`self.winParicle`))
      (bind _asfygame_instance (cast `/Game/Blueprints/FYGameInstance` (`GameplayStatics.GetGameInstance`)))
      (if (>= (`/Game/Blueprints/FYGameInstance.gGameRandomTimes` _asfygame_instance) 10)
        (bind _returnvalue_3 (`GameplayStatics.GetActorOfClass` "/Game/Blueprints/tcpActor.tcpActor_C"))
        (bind _asfygame_instance_2 (cast `/Game/Blueprints/FYGameInstance` (`GameplayStatics.GetGameInstance`)))
        (`/Game/Blueprints/tcpActor.updateTime` _returnvalue_3 (`/Game/Blueprints/FYGameInstance.gPlayerName` _asfygame_instance_2) (`/Game/Blueprints/FYGameInstance.gPlayerTime` _asfygame_instance_2)))))
  (`KismetArrayLibrary.Array_Clear` _rotatearray)
  (set `self.centerPos` (0.0 0.0 0.0)))

(fn `setRotateArray`
  (bind _rotatevalue (`self.rotateValue`))
  (for _array_element (`self.cubeArray`)
    (switch `int` (`self.rotateFrag`)
      (:`0`
        (bind (_returnvalue_x _returnvalue_y _returnvalue_z) (`KismetMathLibrary.BreakVector` (`SceneComponent.K2_GetComponentLocation` (`/Game/Blueprints/FYOneCube.Cube` _array_element))))
        (if (< (`KismetMathLibrary.Abs` (- _rotatevalue _returnvalue_x)) 1.0)
          (`KismetArrayLibrary.Array_Insert` (`self.rotateArray`) _array_element :!label _label)
          (set `self.centerPos` (+ (`self.centerPos`) (`SceneComponent.K2_GetComponentLocation` (`/Game/Blueprints/FYOneCube.Cube` _array_element))))))
      (:`1`
        (if (< (`KismetMathLibrary.Abs` (- _returnvalue_y _rotatevalue)) 1.0)
          (goto _label)))
      (:`2`
        (if (< (`KismetMathLibrary.Abs` (- _returnvalue_z _rotatevalue)) 1.0)
          (goto _label)))))
  (set `self.centerPos` (/ (`self.centerPos`) (`KismetArrayLibrary.Array_Length` (`self.rotateArray`)))))

(fn `startRotateCube`
  (params (rotateFrag :type Integer) (rotateDirection :type Boolean) (rotateLineNum :type Integer))
  (bind _distance (`self.distance`))
  (`GameplayStatics.PlaySound2D` "/Game/Blueprints/Media/rotate.rotate" 1.0 1.0 0.0 null null)
  (if (not (`self.bIsRotating`))
    (set `self.bIsRotating` true)
    (set `self.angleSelf` 0.0)
    (set `self.rotateFrag` rotateFrag)
    (switch `int` rotateLineNum
      (:`0`
        (set `self.rotateValue` _distance))
      (:`1`
        (set `self.rotateValue` 0.0))
      (:`2`
        (set `self.rotateValue` (- 0.0 _distance))))
    (if (== rotateDirection true)
      (set `self.mRotateDirection` 1)
      (else
        (set `self.mRotateDirection` -1)))))

(fn `touchRotate`
  (bind _touchposdistance (`self.touchPosDistance`))
  (bind (_returnvalue_x _returnvalue_y _returnvalue_z) (`KismetMathLibrary.BreakVector` (`self.K2_GetActorLocation` (`|GetArrayItem` (`self.touchArray`) 1))))
  (bind (_returnvalue_x_2 _returnvalue_y_2 _returnvalue_z_2) (`KismetMathLibrary.BreakVector` (`self.K2_GetActorLocation` (`|GetArrayItem` (`self.touchArray`)))))
  (bind _rotatedirection (`/Game/Blueprints/FYOneCube.rotateDirection` (`|GetArrayItem` (`self.touchArray`))))
  (if (< (`KismetArrayLibrary.Array_Length` (`self.touchArray`)) 2)
    (`self.clearTouchArray` :!label _label)
    (elif (== (`/Game/Blueprints/FYOneCube.rotateDirection` (`|GetArrayItem` (`self.touchArray`) 1)) _rotatedirection)
      (if (< (`KismetMathLibrary.Abs` (- _returnvalue_x_2 _returnvalue_x)) 1.0)
        (if (!= _rotatedirection 0)
          (set `self.touchRotateFrag` 0)
          (set `self.touchPosDistance` _returnvalue_x_2)
          (if (`KismetMathLibrary.NearlyEqual_FloatFloat` (`self.touchPosDistance`) 0.0 1.0) :!label _label_2
            (set `self.touchRotateLineNum` 1)
            (bind _newparam (`self.getTouchRotateDirection` :!label _label_3))
            (`self.startRotateCube` (`self.touchRotateFrag`) _newparam (`self.touchRotateLineNum`))
            (`self.clearTouchArray`)
            (elif (< _touchposdistance 0.0)
              (set `self.touchRotateLineNum` 2)
              (goto _label_3)
              (elif (> _touchposdistance 0.0)
                (set `self.touchRotateLineNum` 0)
                (goto _label_3))))
          (else
            (if (< (`KismetMathLibrary.Abs` (- _returnvalue_y_2 _returnvalue_y)) 1.0) :!label _label_4
              (if (!= _rotatedirection 1)
                (set `self.touchRotateFrag` 1)
                (set `self.touchPosDistance` _returnvalue_y_2)
                (goto _label_2)
                (else
                  _)))
            (if (< (`KismetMathLibrary.Abs` (- _returnvalue_z_2 _returnvalue_z)) 1.0)
              (set `self.touchRotateFrag` 2)
              (set `self.touchPosDistance` _returnvalue_z_2)
              (goto _label_2))))
        (else
          (goto _label_4)))
      (else
        (goto _label)))))

(fn `UserConstructionScript`
  (for _index (range 3)
    (for _index_2 (range 3)
      (for _index_3 (range 3)
        (bind _startposition (`self.getStartPosition` 0 _index))
        (bind _startposition_2 (`self.getStartPosition` 1 _index_2))
        (bind _startposition_3 (`self.getStartPosition` 2 _index_3))
        (bind _returnvalue (`AddComponent|NODE_AddChildActorComponent-3`))
        (bind _asfyone_cube (cast `/Game/Blueprints/FYOneCube` (`ChildActorComponent.ChildActor` _returnvalue)))
        (`SceneComponent.K2_SetRelativeLocation` _returnvalue (+ _startposition_3 _startposition_2 _startposition) false false)
        (`SceneComponent.SetWorldScale3D` _returnvalue (`KismetMathLibrary.Conv_DoubleToVector` (`self.allScale`)))
        (`KismetArrayLibrary.Array_Add` (`self.cubeArray`) _asfyone_cube))))
  (for _array_element (`self.cubeArray`)
    (for _array_element_2 (`SceneComponent.GetChildrenComponents` (`/Game/Blueprints/FYOneCube.Cube` _array_element) false)
      (bind `_as子actor组件` (cast `ChildActorComponent` _array_element_2))
      (bind _asfyone_face (cast `/Game/Blueprints/FYOneFace` (`ChildActorComponent.ChildActor` `_as子actor组件`)))
      (`/Game/Blueprints/FYOneFace.setPlaneMaterial` _asfyone_face)))
  (`self.randomRotate`))