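; FYOneFace is a touchable face plane on an FYOneCube piece of what appears to be a Rubik's-style puzzle cube.
; Touch begin and end flag the parent piece, set its rotation axis from the dominant cube-to-plane offset, and queue it in BP_ARTweakCube's TouchArray.
; Touch end then calls TouchRotate on that manager.
; SetPlaneMaterial assigns one of six materials to outward faces, judged by parent component rotation and piece position sign.
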(event `self.Plane.OnInputTouchBegin`
  (params (FingerIndex :type "ETouchIndex Enum" :default "Touch1") (TouchedComponent :type "PrimitiveComponent Object Reference"))
  (bind _asfyone_cube (cast `/Game/Blueprints/FYOneCube` (`self.GetAttachParentActor`)))
  (set `/Game/Blueprints/FYOneCube.isTouched` true _asfyone_cube)
  (`self.setRotateDirection` _asfyone_cube)
  (bind _returnvalue (`GameplayStatics.GetActorOfClass` "/Game/Blueprints/BP_ARTweakCube.BP_ARTweakCube_C"))
  (`KismetArrayLibrary.Array_Insert` (`/Game/Blueprints/BP_ARTweakCube.touchArray` _returnvalue) _asfyone_cube))

(event `self.Plane.OnInputTouchEnd`
  (params (FingerIndex :type "ETouchIndex Enum" :default "Touch1") (TouchedComponent :type "PrimitiveComponent Object Reference"))
  (bind _asfyone_cube (cast `/Game/Blueprints/FYOneCube` (`self.GetAttachParentActor`)))
  (set `/Game/Blueprints/FYOneCube.isTouched` true _asfyone_cube)
  (`self.setRotateDirection` _asfyone_cube)
  (bind _returnvalue (`GameplayStatics.GetActorOfClass` "/Game/Blueprints/BP_ARTweakCube.BP_ARTweakCube_C"))
  (bind _toucharray (`/Game/Blueprints/BP_ARTweakCube.touchArray` _returnvalue))
  (if (!= _asfyone_cube (`|GetArrayItem` _toucharray))
    (`KismetArrayLibrary.Array_Insert` _toucharray _asfyone_cube))
  (`/Game/Blueprints/BP_ARTweakCube.touchRotate` _returnvalue))

(fn `setPlaneMaterial`
  (locals (localParentPosX :type "Float (double-precision)") (localParentPosY :type "Float (double-precision)") (localParentPosZ :type "Float (double-precision)") (localSelfRotateX :type "Float (double-precision)") (localSelfRotateY :type "Float (double-precision)") (localSelfRotateZ :type "Float (double-precision)"))
  (bind _localselfrotatey (`local.localSelfRotateY`))
  (bind (_returnvalue_roll _returnvalue_pitch _returnvalue_yaw) (`KismetMathLibrary.BreakRotator` (`SceneComponent.K2_GetComponentRotation` (`self.GetParentComponent`))))
  (bind _asfyone_cube (cast `/Game/Blueprints/FYOneCube` (`ActorComponent.GetOwner` (`self.GetParentComponent`))))
  (bind (_returnvalue_x _returnvalue_y _returnvalue_z) (`KismetMathLibrary.BreakVector` (`SceneComponent.K2_GetComponentLocation` (`/Game/Blueprints/FYOneCube.Cube` _asfyone_cube))))
  (set `local.localParentPosX` _returnvalue_x)
  (set `local.localParentPosY` _returnvalue_y)
  (set `local.localParentPosZ` _returnvalue_z)
  (set `local.localSelfRotateX` _returnvalue_roll)
  (set `local.localSelfRotateY` _returnvalue_pitch)
  (set `local.localSelfRotateZ` _returnvalue_yaw)
  (if (and (== (`local.localSelfRotateY`) -90.0) (> (`local.localParentPosX`) 0.0))
    (`PrimitiveComponent.SetMaterial` (`self.Plane`) 0 (`self.material1`))
    (elif (and (== (`local.localSelfRotateY`) 90.0) (< (`local.localParentPosX`) 0.0))
      (`PrimitiveComponent.SetMaterial` (`self.Plane`) 0 (`self.material2`))
      (elif (and (`KismetMathLibrary.NearlyEqual_FloatFloat` (`local.localSelfRotateX`) 90.0 0.1) (> (`local.localParentPosY`) 0.0))
        (`PrimitiveComponent.SetMaterial` (`self.Plane`) 0 (`self.material3`))
        (elif (and (`KismetMathLibrary.NearlyEqual_FloatFloat` (`local.localSelfRotateX`) -90.0 0.1) (< (`local.localParentPosY`) 0.0))
          (`PrimitiveComponent.SetMaterial` (`self.Plane`) 0 (`self.material4`))
          (elif (and (== (`KismetMathLibrary.MakeVector` (`local.localSelfRotateX`) (`local.localSelfRotateY`) (`local.localSelfRotateZ`)) (0.0 0.0 0.0)) (> (`local.localParentPosZ`) 0.0))
            (`PrimitiveComponent.SetMaterial` (`self.Plane`) 0 (`self.material5`))
            (elif (and (and (!= _localselfrotatey 0.0) (`KismetMathLibrary.NearlyEqual_FloatFloat` _localselfrotatey 0.0 1.0)) (< (`local.localParentPosZ`) 0.0))
              (`PrimitiveComponent.SetMaterial` (`self.Plane`) 0 (`self.material6`)))))))))

(fn `setRotateDirection`
  (params (NewParam :type "Object Object Reference"))
  (bind _asfyone_cube (cast `/Game/Blueprints/FYOneCube` NewParam))
  (bind _returnvalue (- (`SceneComponent.K2_GetComponentLocation` (`/Game/Blueprints/FYOneCube.Cube` _asfyone_cube)) (`SceneComponent.K2_GetComponentLocation` (`self.Plane`))))
  (bind _output_get (set `self.NewVar_0` _returnvalue))
  (bind _returnvalue_2 (`KismetMathLibrary.Vector_GetAbsMax` _returnvalue))
  (if (== (`KismetMathLibrary.Abs` (.x _output_get)) _returnvalue_2)
    (set `/Game/Blueprints/FYOneCube.rotateDirection` 0 _asfyone_cube)
    (elif (== (`KismetMathLibrary.Abs` (.y _output_get)) _returnvalue_2)
      (set `/Game/Blueprints/FYOneCube.rotateDirection` 1 _asfyone_cube)
      (else
        (set `/Game/Blueprints/FYOneCube.rotateDirection` 2 _asfyone_cube)))))

(fn `UserConstructionScript`)