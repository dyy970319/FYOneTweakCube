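; FYTweakCubePawn is a Blueprint, named as a pawn for FYTweakCubeMap, whose graph currently has no gameplay effect.
; BeginPlay compares the current level name to FYTweakCubeMap, but the branch does nothing; Tick, overlap and construction script are empty.
; Disconnected leftovers would scale a world location to a fixed radius around the origin, rotate toward a variable target, and deactivate a component.
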(event `self.ReceiveBeginPlay`
  (bind _returnvalue (`GameplayStatics.GetCurrentLevelName` true))
  (if (`KismetStringLibrary.EqualEqual_StrStr` _returnvalue "FYTweakCubeMap")
    _))

(event `self.ReceiveTick`
  (params (DeltaSeconds :type "Float (single-precision)")))

(fn `UserConstructionScript`)